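; Tank_BP is the player-controllable tank pawn, wiring its components and input together.
; On BeginPlay it initialises the aiming component with barrel and turret, the movement component with both tracks, and links itself to its HealthBar widget.
; Aim axes rotate the azimuth gimbal and spring arm to orbit the camera, while move, turn and fire inputs forward to the movement and aiming components.
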(event EventBeginPlay
  (Class|TankAmingComponent|Initialise (Variables|Default|GetTankAming) (Variables|Default|GetBarrel) (Variables|Default|GetTurret))
  (Class|TankMovementComponent|Initialise (Variables|Default|GetTankMovement) (Variables|Default|GetTrack_Left) (Variables|Default|GetTrack_Right))
  (CallFunction|InitialiseHealthBarwidget))

(event Input|ActionEvents|InputActionFire
  (params (Key :type Key%20Structure))
  ;[1 1 1] Aim Input Binding
  (:Pressed
    (Class|TankAmingComponent|Fire (Variables|Default|GetTankAming))))

(event Input|AxisEvents|InputAxisAimAzimuth
  (params (AxisValue :type Float%20%28single-precision%29))
  ;[1 1 1] Aim Input Binding
  (Transformation|AddLocalRotation (Variables|Default|GetAzimuth%20Gimbal) (Math|Rotator|MakeRotator 0.0 0.0 AxisValue) false false))

(event Input|AxisEvents|InputAxisAimElevation
  (params (AxisValue :type Float%20%28single-precision%29))
  ;[1 1 1] Aim Input Binding
  (Transformation|AddLocalRotation (Variables|Default|GetSpringArm) (Math|Rotator|MakeRotator 0.0 AxisValue 0.0) false false))

(event Input|AxisEvents|InputAxisMoveForward
  (params (AxisValue :type Float%20%28single-precision%29))
  ;[1 1 1] Movement Input Binding
  (Class|TankMovementComponent|IntendMoveForward (Variables|Default|GetTankMovement) AxisValue))

(event Input|AxisEvents|InputAxisTurnRIght
  (params (AxisValue :type Float%20%28single-precision%29))
  ;[1 1 1] Movement Input Binding
  (Class|TankMovementComponent|IntendTurnRight (Variables|Default|GetTankMovement) AxisValue))

(fn ConstructionScript
  (Development|PrintString "DONKEY:Tank_BP Construct"))

(fn InitialiseHealthBarwidget
  (bind _ashealth_bar (Utilities|Casting|CastToHealthBar (UserInterface|GetUserWidgetObject (Variables|Default|GetWidget))))
  (Variables|/Game/Blueprints/HealthBar.HealthBar_C|SetMyTank _ashealth_bar self)
  (return))